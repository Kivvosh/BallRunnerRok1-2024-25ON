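; BP_win_volume is a level exit trigger that completes the level when an actor passing the BabaIsYou check overlaps its box.
; If any BP_Crystal_01 actors remain, it only prints a Polish message that not all gems were collected.
; Otherwise it fades the camera out, waits, then opens the level following the current one in the TabLvlNames01 name array.
; On the array's last level it prints a final-level message instead.
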(event OnComponentBeginOverlap(Box)
  (params (OverlappedComponent :type Primitive%20Component%20Object%20Reference) (OtherActor :type Actor%20Object%20Reference) (OtherComp :type Primitive%20Component%20Object%20Reference) (OtherBodyIndex :type Integer) (bFromSweep :type Boolean) (SweepResult :type Hit%20Result%20Structure%20%28by%20ref%29))
  (Utilities|BabaIsYou OtherActor
    (:true
      (bind _outactors (Actor|GetAllActorsOfClass "/Game/Blueprints/BP_Crystal_01.BP_Crystal_01_C"))
      (if (> (Utilities|Array|Length _outactors) 0)
        (Development|PrintString "Nie zebrano wszystkich klejnotów.")
        (else
          (CameraFades|StartCameraFade :self (Game|GetPlayerCameraManager 0) :ToAlpha 1.0 :Duration 1.0 :bHoldWhenFinished true)
          (Utilities|FlowControl|Delay 1.0)
          (CallFunction|CompleteLvl))))))

(fn ConstructionScript)

(fn GetCurrentLvlIndex
  (bind _returnvalue (Game|GetCurrentLevelName true))
  (return (Utilities|Array|FindItem (Variables|Default|Gettab_lvl_names_01) _returnvalue)))

(fn GetNextLvlName
  (bind _returnvalue (CallFunction|GetCurrentLvlIndex))
  (return (Utilities|Array|Get(acopy) (Variables|Default|Gettab_lvl_names_01) (+ _returnvalue 1))))

(fn LoadNextLvl
  (bind _output (CallFunction|GetNextLvlName))
  (Game|OpenLevel(byName) (Utilities|String|StringToName _output)))

(fn IsFinalLevel
  (bind _returnvalue (CallFunction|GetCurrentLvlIndex))
  (return (== (Utilities|Array|LastIndex (Variables|Default|Gettab_lvl_names_01)) _returnvalue)))

(fn CompleteLvl
  (bind _returnvalue (CallFunction|IsFinalLevel))
  (if _returnvalue
    (Development|PrintString "OSTATNI POZIOM")
    (else
      (CallFunction|LoadNextLvl))))